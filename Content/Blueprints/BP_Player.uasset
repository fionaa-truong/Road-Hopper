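; Player actor for a Frogger-style road-crossing game that hops in grid steps, scores by furthest row reached, and wins at a set Y distance.
; Each input shifts a cumulative target location, so rapid presses queue, and a per-direction timeline lerps the actor toward it.
; Finished forward hops update the score in GM_RoadHopper and check for a win.
; Overlapping a BP_Car ends the game, disables input and destroys the player.
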(event OnComponentBeginOverlap(Box)
  (params (OverlappedComponent :type Primitive%20Component%20Object%20Reference) (OtherActor :type Actor%20Object%20Reference) (OtherComp :type Primitive%20Component%20Object%20Reference) (OtherBodyIndex :type Integer) (bFromSweep :type Boolean) (SweepResult :type Hit%20Result%20Structure%20%28by%20ref%29))
  ;[1 1 1] Lose Condition - when the vehicle and player overlap
  (Utilities|Casting|CastToBP_Car OtherActor)
  (bind _asgm_road_hopper (Utilities|Casting|CastToGM_RoadHopper (Game|GetGameMode)))
  ;;[1 1 1] Set IsGameOver to be TRUE
  (Variables|/Game/Blueprints/GM_RoadHopper.GM_RoadHopper_C|SetIsGameOver _asgm_road_hopper true)
  ;;[1 1 1] Prevents the player from moving after losing
  (Audio|Components|Audio|Stop (Variables|Default|GetInterpolateForward))
  ;;[1 1 1] Retrieves the players score when they die to print
  (Development|PrintString (Utilities|String|Append "Game Over! Final Score: " (Utilities|String|ToString(Integer) (Variables|/Game/Blueprints/GM_RoadHopper.GM_RoadHopper_C|GetPlayerScore _asgm_road_hopper))))
  ;;[1 1 1] Disable user input and destory the character once the player and a vehicle collide
  (Input|DisableInput (Game|GetPlayerController 0))
  (Actor|DestroyActor))

(event EventBeginPlay
  ;[1 1 1] Sets the origin location to the player's initial location when the game starts
  (Variables|Default|SetOriginLoc (Transformation|GetActorLocation)))

(event Collision|EventActorBeginOverlap
  (params (OtherActor :type Actor%20Object%20Reference)))

(event EventTick
  (params (DeltaSeconds :type Float%20%28single-precision%29)))

(event Input|ActionEvents|InputActionMoveForward
  (params (Key :type Key%20Structure :default "None"))
  ;[1 1 1] Forward Movement Input, Increment Score, and Win Condition
  (:Pressed
    (CallFunction|MoveForward)
    ;;[1 1 1] Interpolate movement using for smooth movement and to prevent teleportation
    (bind _forward (Timeline|InterpolateForward PlayFromStart)
      (:Update
        (Transformation|SetActorLocation (Math|Vector|Lerp(Vector) (Variables|Default|GetStartingLoc) (Variables|Default|GetEndingLoc) _forward) false false))
      (:Finished
        (bind _asgm_road_hopper (Utilities|Casting|CastToGM_RoadHopper (Game|GetGameMode)))
        (bind _output_get (Variables|Default|SetCurRow (Math|Float|Round (/ (- (.Y (Math|Vector|BreakVector (Variables|Default|GetEndingLoc))) (.Y (Math|Vector|BreakVector (Variables|Default|GetOriginLoc)))) 1e+02))))
        (if (> _output_get (Variables|Default|GetMaxRowReached))
          (bind _output_get_2 (Variables|Default|SetMaxRowReached (Variables|Default|GetCurRow)))
          (Variables|/Game/Blueprints/GM_RoadHopper.GM_RoadHopper_C|SetPlayerScore _asgm_road_hopper _output_get_2)
          (if (>= (Math|Float|Truncate (.Y (Math|Vector|BreakVector (Variables|Default|GetEndingLoc)))) 6000)
            (Variables|/Game/Blueprints/GM_RoadHopper.GM_RoadHopper_C|SetIsGameOver _asgm_road_hopper true)
            (Development|PrintString (Utilities|String|Append "You Win! Score: " (Utilities|String|ToString(Integer) (Variables|/Game/Blueprints/GM_RoadHopper.GM_RoadHopper_C|GetPlayerScore _asgm_road_hopper))))
            (Variables|/Game/Blueprints/GM_RoadHopper.GM_RoadHopper_C|SetIsGameOver _asgm_road_hopper true)
            (Input|DisableInput (Game|GetPlayerController 0))))))))

(event Input|ActionEvents|InputActionMoveBackward
  (params (Key :type Key%20Structure :default "None"))
  ;[1 1 1] Backward Movement Input
  (:Pressed
    (CallFunction|MoveBackward)
    (bind _forward (Timeline|InterpolateBackwards PlayFromStart)
      (:Update
        (Transformation|SetActorLocation (Math|Vector|Lerp(Vector) (Variables|Default|GetStartingLoc) (Variables|Default|GetEndingLoc) _forward) false false)))))

(event Input|ActionEvents|InputActionMoveLeft
  (params (Key :type Key%20Structure :default "None"))
  ;[1 1 1] Left Movement Input
  (:Pressed
    (CallFunction|MoveLeft)
    (bind _forward (Timeline|InterpolateLeft PlayFromStart)
      (:Update
        (Transformation|SetActorLocation (Math|Vector|Lerp(Vector) (Variables|Default|GetStartingLoc) (Variables|Default|GetEndingLoc) _forward) false false)))))

(event Input|ActionEvents|InputActionMoveRight
  (params (Key :type Key%20Structure :default "None"))
  ;[1 1 1] Right Movement Input
  (:Pressed
    (CallFunction|MoveRight)
    (bind _forward (Timeline|InterpolateRight PlayFromStart)
      (:Update
        (Transformation|SetActorLocation (Math|Vector|Lerp(Vector) (Variables|Default|GetStartingLoc) (Variables|Default|GetEndingLoc) _forward) false false)))))

(fn ConstructionScript
  (Components|StaticMesh|SetStaticMesh (Variables|Default|GetBody) (Variables|Default|GetBodyModel))
  (Components|StaticMesh|SetStaticMesh (Variables|Default|GetHead) (Variables|Default|GetHeadModel)))

(fn MoveForward
  ;[1 1 1] Move forward by getting the player's current location, moving 100 units on the y-axis from the ending location at the time the movement key is pressed (to allow multiple inputs to be taken in within a short time span without disrupting the movement), and then setting it to be the ending location.
  (Variables|Default|SetStartingLoc (Transformation|GetActorLocation))
  (Variables|Default|SetEndingLoc (+ (Variables|Default|GetEndingLoc) "0,100.000000, 0")))

(fn MoveBackward
  ;[1 1 1] Move backward by getting the player's current location, moving -100 units on the y-axis from the ending location at the time the movement key is pressed (to allow multiple inputs to be taken in within a short time span without disrupting the movement), and then setting it to be the ending location.
  (Variables|Default|SetStartingLoc (Transformation|GetActorLocation))
  (Variables|Default|SetEndingLoc (+ (Variables|Default|GetEndingLoc) "0,-100.000000, 0")))

(fn MoveLeft
  ;[1 1 1] Move left by getting the player's current location, moving 100 units on the x-axis from the ending location at the time the movement key is pressed (to allow multiple inputs to be taken in within a short time span without disrupting the movement), and then setting it to be the ending location.
  (Variables|Default|SetStartingLoc (Transformation|GetActorLocation))
  (Variables|Default|SetEndingLoc (+ (Variables|Default|GetEndingLoc) "100.000000,-0.000000, 0")))

(fn MoveRight
  ;[1 1 1] Move right by getting the player's current location, moving -100 units on the x-axis from the ending location at the time the movement key is pressed (to allow multiple inputs to be taken in within a short time span without disrupting the movement), and then setting it to be the ending location.
  (Variables|Default|SetStartingLoc (Transformation|GetActorLocation))
  (Variables|Default|SetEndingLoc (+ (Variables|Default|GetEndingLoc) "-100.000000,0.000000, 0")))